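; BP_barricade is a procedural barricade actor that builds a row of static meshes between FenceStart and FenceEnd.
; The construction script divides that distance by Length to set the piece count, then spaces meshes along the direction from the actor's origin, skipping index zero.
; Each piece faces along the line with slight random roll, yaw and height scale, for an irregular look.
; The event graph has no active logic.
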(event EventBeginPlay)

(event Collision|EventActorBeginOverlap
  (params (OtherActor :type Actor%20Object%20Reference)))

(event EventTick
  (params (DeltaSeconds :type Float%20%28single-precision%29)))

(fn ConstructionScript
  (bind _fencestart (Variables|Default|GetFenceStart))
  (bind _fenceend (Variables|Default|GetFenceEnd))
  (bind _returnvalue (Math|Vector|GetUnitDirection(Vector) _fencestart _fenceend))
  (for _index (range 1 (- (Math|Float|Truncate (/ (Math|Vector|VectorLength (- (Variables|Default|GetFenceEnd) (Variables|Default|GetFenceStart))) (Variables|Default|GetLength))) 1))
    (AddComponent|AddStaticMeshComponent false (Math|Transform|MakeTransform (* _index (Variables|Default|GetLength) _returnvalue) (Math|Rotator|CombineRotators (Math|Conversions|RotationFromXVector _returnvalue) (Math|Rotator|MakeRotator (Math|Random|RandomFloatinRange -1e+01 1e+01) 0.0 (Math|Random|RandomFloatinRange -1e+01 1e+01))) (Math|Vector|MakeVector 1.0 1.0 (Math|Random|RandomFloatinRange 0.9 1.0))))))