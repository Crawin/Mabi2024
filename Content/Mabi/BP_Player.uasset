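; Player character Blueprint with HUD, weapon pickup, melee attacks and HP/EXP stats.
; Capsule overlaps attach items to hand sockets matched by display name, which also selects each click's MT_Paladin montage section; G drops the right-hand item.
; Mesh overlaps deal damage; death cuts EXP and teleports to the start point at full HP.
; EXP gain and IOCP connection are unwired, though EndPlay still disconnects IOCP.
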(event OnComponentBeginOverlap(CapsuleComponent)
  (params (OverlappedComponent :type Primitive%20Component%20Object%20Reference) (OtherActor :type Actor%20Object%20Reference) (OtherComp :type Primitive%20Component%20Object%20Reference) (OtherBodyIndex :type Integer) (bFromSweep :type Boolean) (SweepResult :type Hit%20Result%20Structure%20%28by%20ref%29))
  (if (not (== OtherActor self))
    (bind (_left_ _socket) (CallFunction|WeaponType OtherActor))
    (if _left_
      (Utilities|IsValid (Variables|Default|GetLeftGrabbed)
        (:Is%20Not%20Valid
          (bind _output_get (Variables|Default|SetLeftGrabbed OtherActor))
          (Class|Handle|Grab(Message) _output_get)))
      (else
        (Utilities|IsValid (Variables|Default|GetRightGrabbed)
          (:Is%20Not%20Valid
            (bind _output_get_2 (Variables|Default|SetRightGrabbed OtherActor))
            (Class|Handle|Grab(Message) _output_get_2)))))
    (Transformation|AttachComponentToComponent OtherActor (Variables|Character|GetMesh) _socket "SnapToTarget" "SnapToTarget" "KeepRelative" true)))

(event OnComponentBeginOverlap(Mesh)
  (params (OverlappedComponent :type Primitive%20Component%20Object%20Reference) (OtherActor :type Actor%20Object%20Reference) (OtherComp :type Primitive%20Component%20Object%20Reference) (OtherBodyIndex :type Integer) (bFromSweep :type Boolean) (SweepResult :type Hit%20Result%20Structure%20%28by%20ref%29))
  (bind _self self)
  (if (not (== OtherActor _self))
    (Game|Damage|ApplyDamage OtherActor 1.0 0 _self)))

(event Input|EnhancedActionEvents|EnhancedInputActionLEFTCLICK
  (params (ActionValue :type Boolean) (ElapsedSeconds :type Float%20%28double-precision%29) (TriggeredSeconds :type Float%20%28double-precision%29) (InputAction :type Input%20Action%20Object%20Reference :default "/Game/Mabi/Input/LEFTCLICK.LEFTCLICK"))
  (if (not (Variables|Default|GetPlayingMontage?))
    (Variables|Default|SetPlayingMontage? true)
    (bind _weaponname (CallFunction|LeftWeaponType))
    (Animation|Montage|PlayMontage (Variables|Character|GetMesh) "/Game/Assets/Human/Animations/MT_Paladin.MT_Paladin" 1.0 0.0 _weaponname
      (:OnCompleted
        (Variables|Default|SetPlayingMontage? false)))))

(event Input|EnhancedActionEvents|EnhancedInputActionRIGHTCLICK
  (params (ActionValue :type Boolean) (ElapsedSeconds :type Float%20%28double-precision%29) (TriggeredSeconds :type Float%20%28double-precision%29) (InputAction :type Input%20Action%20Object%20Reference :default "/Game/Mabi/Input/RIGHTCLICK.RIGHTCLICK"))
  (if (not (Variables|Default|GetPlayingMontage?))
    (Variables|Default|SetPlayingMontage? true)
    (bind _weaponname (CallFunction|RightWeaponType))
    (Animation|Montage|PlayMontage (Variables|Character|GetMesh) "/Game/Assets/Human/Animations/MT_Paladin.MT_Paladin" 1.0 0.0 _weaponname
      (:OnCompleted
        (Variables|Default|SetPlayingMontage? false)))))

(event EventEndPlay
  (params (EndPlayReason :type EEndPlayReason%20Enum :default "Destroyed"))
  (Widget|RemovefromParent (Variables|Default|GetPlayerUI))
  (Class|IOCP|DisconnectIOCP (Variables|Default|GetIOCP)))

(event EventBeginPlay
  (bind _returnvalue (Game|ConstructObjectfromClass "/Game/Mabi/UI_Player.UI_Player_C" self))
  (bind _output_get (Variables|Default|SetPlayerUI _returnvalue))
  (UserInterface|Viewport|AddtoViewport _output_get 0)
  (CallFunction|InitStatus)
  (Variables|Default|SetStartPos (Transformation|GetWorldLocation (Variables|Collision|GetCapsuleComponent))))

(event Game|Damage|EventAnyDamage
  (params (Damage :type Float%20%28single-precision%29) (DamageType :type Damage%20Type%20Object%20Reference) (InstigatedBy :type Controller%20Object%20Reference) (DamageCauser :type Actor%20Object%20Reference))
  (if (not (== DamageCauser self))
    (CallFunction|UpdateHPPercent Damage)))

(event Input|KeyboardEvents|Q
  (params (Key :type Key%20Structure :default "None")))

(event Input|KeyboardEvents|G
  (params (Key :type Key%20Structure :default "None"))
  (:Pressed
    (Utilities|IsValid (Variables|Default|GetRightGrabbed)
      (:Is%20Valid
        (Transformation|DetachFromActor (Variables|Default|GetRightGrabbed) "KeepWorld" "KeepRelative" "KeepRelative")
        (Class|Handle|Drop(Message) (Variables|Default|GetRightGrabbed))
        (Variables|Default|SetRightGrabbed 0)))))

(fn ConstructionScript)

(fn RightWeaponType
  (bind _rightgrabbed (Variables|Default|GetRightGrabbed))
  (bind _returnvalue (Utilities|GetDisplayName _rightgrabbed))
  (if (Utilities|String|Contains _returnvalue "Axe")
    (return "Axe")
    (elif (Utilities|String|Contains _returnvalue "Sword")
      (return "Sword")
      (else
        (return "RightPunch")))))

(fn LeftWeaponType
  (if (Utilities|String|Contains (Utilities|GetDisplayName (Variables|Default|GetLeftGrabbed)) "Shield")
    (return "Shield")
    (else
      (return "LeftPunch"))))

(fn WeaponType
  (params (Weapon :type Actor%20Object%20Reference))
  (bind _returnvalue (Utilities|GetDisplayName Weapon))
  (if (Utilities|String|Contains _returnvalue "Shield")
    (return true "Shield")
    (elif (Utilities|String|Contains _returnvalue "Sword")
      (return false "Sword")
      (elif (Utilities|String|Contains _returnvalue "Axe")
        (return false "Axe")))))

(fn InitStatus
  (Variables|Default|SetLevel 1)
  (Variables|Default|SetMaxEXP 1e+02)
  (Variables|Default|SetEXP 0.0)
  (Variables|Default|SetMaxHP 1e+02)
  (Variables|Default|SetHP 1e+02))

(fn UpdateEXPPercent
  (if (>= (- (Variables|Default|GetEXP) (Variables|Default|GetMaxEXP)) 0.0)
    ;[1 1 1] Level up
    (Math|Integer|IncrementInt (Variables|Default|GetLevel)
      (:%20%20
        (Variables|Default|SetEXP (- (Variables|Default|GetEXP) (Variables|Default|GetMaxEXP)))
        (Variables|Default|SetMaxEXP (* (Variables|Default|GetMaxEXP) 2.0))))))

(fn UpdateHPPercent
  (params (Damage :type Float%20%28double-precision%29))
  (if (<= (- (Variables|Default|GetHP) Damage) 0.0)
    (Variables|Default|SetEXP (* (Variables|Default|GetEXP) 0.9))
    (Variables|Default|SetHP 1e+02)
    (Transformation|SetWorldLocation (Variables|Collision|GetCapsuleComponent) (Variables|Default|GetStartPos) false false)
    (else
      (Variables|Default|SetHP (- (Variables|Default|GetHP) Damage)))))